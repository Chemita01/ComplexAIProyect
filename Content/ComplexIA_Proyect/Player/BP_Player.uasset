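; BP_Player is a click-selectable unit pawn that can be sent to a destination through AI movement.
; On click, it waits briefly, registers itself with the first player controller through a RegisterActor message, then shows its SelectionMarker.
; ToggleSelect shows or hides that marker, and Goto moves the pawn with AIMoveTo.
; The MoveTo function and construction script are empty.
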(event `self.ReceiveActorOnClicked`
  (params (ButtonPressed :type "Key Structure"))
  (`KismetSystemLibrary.Delay` 0.1)
  (message `/Game/ComplexIA_Proyect/Player/Interfaces/BPI_PlayerController.RegisterActor` (`GameplayStatics.GetPlayerController` 0) self)
  (`self.ToggleSelect` true))

(event `self.ToggleSelect`
  (params (`Select/Deselect` :type Boolean))
  (`SceneComponent.SetHiddenInGame` (`self.SelectionMarker`) (not `Select/Deselect`) false))

(event `/Game/ComplexIA_Proyect/Player/Interfaces/BPI_CharacterMovement.GoTo`
  (params (Destination :type "Vector Structure"))
  (`|AIMoveTo` self Destination null))

(fn `MoveTo`
  (params (Location :type "Vector Structure")))

(fn `UserConstructionScript`)